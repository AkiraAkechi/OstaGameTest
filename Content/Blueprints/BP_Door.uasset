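; BP_Door is an interactable door that other interact actors can unlock but the player cannot open directly.
; When a BP_BaseInteractActor triggers OnInteract, it destroys the BlockPlane component and sets the status text to Open.
; A direct interaction from the player only prints a Blocked message while the plane still exists.
; The plane's validity serves as the door's closed state, so opening happens once.
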(event `InteractInterface.OnInteract`
  (params (Caller :type "Actor Object Reference"))
  (cast `/Game/Blueprints/InteractActors/BP_BaseInteractActor` Caller
    (:`then`
      (bind _blockplane (`self.BlockPlane`)
        (:`then`
          (`ActorComponent.K2_DestroyComponent` _blockplane)
          (`TextRenderComponent.K2_SetText` (`self.StatusText`) (`|FormatText` "Open")))
        (:`else`)))
    (:`CastFailed`
      (if (== Caller (`GameplayStatics.GetPlayerCharacter` 0))
        (`self.BlockPlane`
          (:`then`
            (`/Game/Blueprints/BP_MyFunctionLib.Print Screen Message` "Blocked" 1.0))
          (:`else`))))))

(fn `UserConstructionScript`)