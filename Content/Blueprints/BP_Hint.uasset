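; BP_Hint is a hint actor that shows the look of a randomly chosen actor from its ActorsForHint list.
; Shortly after BeginPlay, it picks a random entry and sets that actor's IsRandomChoosen flag.
; It then copies the first material of the chosen actor's mesh onto its own StaticMesh as the visual clue.
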(event `self.ReceiveBeginPlay`
  (`KismetSystemLibrary.Delay` 5.0)
  (`self.SetRandomSuccessfullActor`))

(event `SetRandomSuccessfullActor`
  (bind _actorsforhint (`self.ActorsForHint`))
  (bind _output_get (set `self.RandomInt` (`KismetMathLibrary.RandomIntegerInRange` 0 (`KismetArrayLibrary.Array_LastIndex` _actorsforhint))))
  (bind _output (`|GetArrayItem` _actorsforhint _output_get))
  (set `/Game/Blueprints/InteractActors/BP_BaseInteractActor.isRandomChoosen` true _output)
  (`PrimitiveComponent.SetMaterial` (`self.StaticMesh`) 0 (`PrimitiveComponent.GetMaterial` (`InteractActor.Mesh` _output) 0)))

(fn `UserConstructionScript`)