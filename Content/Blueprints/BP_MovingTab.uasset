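; BP_MovingTab is an interactable tab whose static mesh shuttles back and forth between two points once an InteractActor triggers it.
; On that interaction, MoveComponentTo eases the mesh to the relative transform of Point1 or Point2, flipping ToSecondPosition and looping endlessly through a Delay of OverTime.
; A direct interaction from the player character only prints a hint that the tab can move.
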(event `InteractInterface.OnInteract`
  (params (Caller :type "Actor Object Reference"))
  (bind (_returnvalue_location _returnvalue_rotation) (`KismetMathLibrary.BreakTransform` (`SceneComponent.GetRelativeTransform` (select `bool` (`self.bToSecondPosition`) :`false` (`self.Point_1`) :`true` (`self.Point_2`)))))
  (cast `InteractActor` Caller
    (:`then`
      (`KismetSystemLibrary.MoveComponentTo` (`self.StaticMesh`) _returnvalue_location _returnvalue_rotation true true (`self.Over Time`) :!label _label)
      (if (`self.bToSecondPosition`)
        (set `self.bToSecondPosition` false)
        (else
          (set `self.bToSecondPosition` true)))
      (`KismetSystemLibrary.Delay` (`self.Over Time`))
      (goto _label))
    (:`CastFailed`
      (if (== Caller (`GameplayStatics.GetPlayerCharacter` 0))
        (`/Game/Blueprints/BP_MyFunctionLib.Print Screen Message` "This Tab can move" 2.0)))))

(fn `UserConstructionScript`)