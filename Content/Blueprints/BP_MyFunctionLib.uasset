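; BP_MyFunctionLib is a Blueprint library of two helper functions for on-screen messages and game mode access.
; PrintScreenMessage creates a WBP_SreenMessage widget with the given text and duration and adds it to the viewport, but only when no top-level instance exists, so overlapping messages are skipped rather than queued.
; GetGameModeBP returns the current game mode cast to SeverstalTestGameMode.
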(fn `GetGameModeBP`
  (returns (`AsSeverstal Test Game Mode` :type "SeverstalTestGameMode Object Reference"))
  (bind _asseverstal_test_game_mode (cast `SeverstalTestGameMode` (`GameplayStatics.GetGameMode` null)))
  (return _asseverstal_test_game_mode))

(fn `Print Screen Message`
  (params (`In Text` :type Text) (Duration :type "Float (double-precision)"))
  (returns (Widget :type "/Game/UI/WBP_SreenMessage Object Reference"))
  (bind _foundwidgets (`WidgetBlueprintLibrary.GetAllWidgetsOfClass` null "/Game/UI/WBP_SreenMessage.WBP_SreenMessage_C"))
  (if (<= (`KismetArrayLibrary.Array_Length` _foundwidgets) 0)
    (bind _returnvalue (`|CreateWidget` "/Game/UI/WBP_SreenMessage.WBP_SreenMessage_C" null `In Text` Duration))
    (`UserWidget.AddToViewport` _returnvalue 0)
    (return _returnvalue)))