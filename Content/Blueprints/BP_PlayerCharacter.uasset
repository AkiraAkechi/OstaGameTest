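; Player character Blueprint that carries a colored key inventory and toggles the pause menu widget.
; Slot 0 is the held key, shown on KeyMesh with a material selected by color.
; Pickups push the held key to the array's end, SetGrabItem swaps a slot into hand, and drops promote the following item.
; Dispatchers broadcast inventory changes and number-key presses.
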(event `InputAction|Pause`
  (params (Key :type "Key Structure"))
  (:`Pressed`
    (bind _pausemenu (`self.PauseMenu`)
      (:`then`
        (`/Game/UI/WBP_PauseMenu.RemoveMenu` _pausemenu)
        (set `self.PauseMenu` null))
      (:`else`
        (bind _returnvalue (`|CreateWidget` "/Game/UI/WBP_PauseMenu.WBP_PauseMenu_C"))
        (bind _output_get (set `self.PauseMenu` _returnvalue))
        (`UserWidget.AddToViewport` _output_get 0)))))

(event `PickUpItem`
  (params (Key :type "EObjectColor Enum" :default "OC_Cyan"))
  (bind _inventoryitems (`self.InventoryItems`))
  (if (or (`self.bGrabItem`) (`KismetArrayLibrary.Array_IsValidIndex` (`self.InventoryItems`)))
    (`KismetArrayLibrary.Array_Set` _inventoryitems (`KismetArrayLibrary.Array_Length` _inventoryitems) (`|GetArrayItem` _inventoryitems) true))
  (`SceneComponent.SetHiddenInGame` (`self.KeyMesh`) false false)
  (`KismetArrayLibrary.Array_Set` (`self.InventoryItems`) 0 Key true)
  (`self.onIventoryItemChanged`)
  (`PrimitiveComponent.SetMaterial` (`self.KeyMesh`) 0 (select `EObjectColor` Key :`OC_Cyan` "/Engine/VREditor/BasicMeshes/MI_Cube_02.MI_Cube_02" :`OC_Magenta` "/Engine/VREditor/BasicMeshes/MI_Pyramid_01.MI_Pyramid_01" :`OC_Yellow` "/Engine/VREditor/BasicMeshes/MI_Cube_01.MI_Cube_01" :`OC_Black` "/Engine/VREditor/BasicMeshes/MI_Floor_01.MI_Floor_01" :`OC_Red` "/Engine/VREditor/BasicMeshes/MI_Cube_03.MI_Cube_03" :`OC_Green` "/Engine/VREditor/BasicMeshes/MI_Green.MI_Green" :`OC_Blue` "/Engine/VREditor/BasicMeshes/MI_Ball_01.MI_Ball_01" :!type "MaterialInterface Object Reference"))
  (set `self.bGrabItem` true))

(event `InputAction|NumberInput`
  (params (Key :type "Key Structure"))
  (:`Pressed`
    (`self.onNumberKeyInput` (`KismetStringLibrary.Conv_StringToInt` (`KismetTextLibrary.Conv_TextToString` (`KismetInputLibrary.Key_GetDisplayName` Key))))))

(event `DropItem`
  (params (Item :type "EObjectColor Enum" :default "OC_Cyan"))
  (bind _inventoryitems (`self.InventoryItems`))
  (bind _returnvalue (`KismetArrayLibrary.Array_Find` _inventoryitems Item))
  (bind _returnvalue_2 (+ _returnvalue 1))
  (`SceneComponent.SetHiddenInGame` (`self.KeyMesh`) true false)
  (set `self.bGrabItem` false)
  (if (`KismetArrayLibrary.Array_IsValidIndex` _inventoryitems _returnvalue_2)
    (`self.SetGrabItem` _returnvalue_2))
  (`KismetArrayLibrary.Array_Remove` (`self.InventoryItems`) _returnvalue)
  (`self.onIventoryItemChanged`))

(fn `SetGrabItem`
  (params (FromSlot :type Integer))
  (locals (ItemToChagePosition :type "EObjectColor Enum") (PreviousItem :type "EObjectColor Enum"))
  (bind _inventoryitems (`self.InventoryItems`))
  (bind _inventoryitems_2 (`self.InventoryItems`))
  (if (`KismetArrayLibrary.Array_IsValidIndex` _inventoryitems FromSlot)
    (set `local.ItemToChagePosition` (`|GetArrayItem` _inventoryitems FromSlot))
    (set `local.PreviousItem` (`|GetArrayItem` (`self.InventoryItems`)))
    (`SceneComponent.SetHiddenInGame` (`self.KeyMesh`) false false)
    (`KismetArrayLibrary.Array_Set` _inventoryitems_2 0 (`local.ItemToChagePosition`))
    (`KismetArrayLibrary.Array_Set` _inventoryitems_2 (`local.FromSlot`) (`local.PreviousItem`))
    (`PrimitiveComponent.SetMaterial` (`self.KeyMesh`) 0 (select `EObjectColor` (`local.ItemToChagePosition`) :`OC_Cyan` "/Engine/VREditor/BasicMeshes/MI_Cube_02.MI_Cube_02" :`OC_Magenta` "/Engine/VREditor/BasicMeshes/MI_Pyramid_01.MI_Pyramid_01" :`OC_Yellow` "/Engine/VREditor/BasicMeshes/MI_Cube_01.MI_Cube_01" :`OC_Black` "/Engine/VREditor/BasicMeshes/MI_Floor_01.MI_Floor_01" :`OC_Red` "/Engine/VREditor/BasicMeshes/MI_Cube_03.MI_Cube_03" :`OC_Green` "/Engine/VREditor/BasicMeshes/MI_Green.MI_Green" :`OC_Blue` "/Engine/VREditor/BasicMeshes/MI_Ball_01.MI_Ball_01" :!type "MaterialInterface Object Reference"))
    (set `self.bGrabItem` true)
    (`self.onIventoryItemChanged`)))

(fn `UserConstructionScript`)