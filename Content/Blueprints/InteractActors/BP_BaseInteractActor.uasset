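; Base interactable actor that triggers its managed actors, either directly or as part of a chain of linked interact actors.
; On BeginPlay it picks a random color, re-rolling on matches with actors earlier in its chain, and applies the mapped material.
; In chain mode, a valid, optionally order-checked interaction is broadcast so each member marks the caller active in its map.
; Managed actors receive chain messages until completion, then the interact message.
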(event `self.ReceiveBeginPlay`
  (set `self.ColorEnumValue` (cast `EObjectColor` (`KismetMathLibrary.Conv_IntToByte` (`KismetMathLibrary.RandomIntegerInRange` (`self.MinRandomIndex`) (`self.MaxRandomIndex`)))))
  (`self.SameColorCheck`)
  (`PrimitiveComponent.SetMaterial` (`self.Mesh`) 0 (`BlueprintMapLibrary.Map_Find` (`self.MaterialMap`) (`self.ColorEnumValue`))))

(event `InteractInterface.ChainInteraction`
  (params (Caller :type "Actor Object Reference"))
  (bind _interactionchain (`self.InteractionChain`))
  (bind _asbp_base_interact_actor (cast `/Game/Blueprints/InteractActors/BP_BaseInteractActor` Caller))
  (bind _keys (`BlueprintMapLibrary.Map_Keys` _interactionchain))
  (if (`KismetArrayLibrary.Array_Contains` _keys _asbp_base_interact_actor)
    (`BlueprintMapLibrary.Map_Add` _interactionchain _asbp_base_interact_actor true)))

(fn `CheckChainOrder`
  (returns (ReturnValue :type Boolean))
  (locals (OrderActors :type "Array of InteractActor Object Reference") (bCorrectValue :type Boolean) (ValueArray :type "Array of Boolean"))
  (bind _interactionchain (`self.InteractionChain`))
  (bind _keys (`BlueprintMapLibrary.Map_Keys` _interactionchain))
  (bind _output_get (set `local.OrderActors` _keys))
  (if (== (`KismetArrayLibrary.Array_Find` _output_get self) 0)
    (return true)
    (else
      (bind _values (`BlueprintMapLibrary.Map_Values` _interactionchain))
      (set `local.ValueArray` _values)
      (for _index (range (`self.InteractionChainIndex`))
        (if (`|GetArrayItem` (`local.ValueArray`) _index)
          (set `local.bCorrectValue` true)
          (else
            (set `local.bCorrectValue` false)
            (break))))
      (if (`local.bCorrectValue`)
        (for _index_2 (range (`self.InteractionChainIndex`) (+ (`KismetArrayLibrary.Array_LastIndex` (`local.OrderActors`)) 1))
          (if (`|GetArrayItem` (`local.ValueArray`) _index_2)
            (set `local.bCorrectValue` false)
            (break)
            (else
              (set `local.bCorrectValue` true))))
        (return (`local.bCorrectValue`))
        (else
          (return false))))))

(fn `CompliteChainCheck`
  (returns (ReturnValue :type Boolean))
  (locals (isChainComplite :type Boolean))
  (bind _values (`BlueprintMapLibrary.Map_Values` (`self.InteractionChain`)))
  (for _array_element _values
    (if _array_element
      (set `local.isChainComplite` true)
      (else
        (set `local.isChainComplite` false)
        (break))))
  (return (`local.isChainComplite`)))

(fn `ResultInteraction`
  (returns (Result :type Boolean))
  (bind (_value _returnvalue) (`BlueprintMapLibrary.Map_Find` (`self.InteractionChain`) self))
  (if (`self.isChainInteraction`)
    (if _returnvalue
      (if _value
        (`KismetSystemLibrary.PrintString` "this actor already active" false)
        (return false)
        (else
          (if (`self.bChairInOrder`)
            (bind _returnvalue_2 (`self.CheckChainOrder`))
            (if _returnvalue_2
              _
              (else
                (return false))))
          (bind _keys (`BlueprintMapLibrary.Map_Keys` (`self.InteractionChain`)))
          (for _array_element _keys
            (message `InteractInterface.ChainInteraction` _array_element self))
          (bind _returnvalue_3 (`self.CompliteChainCheck`))
          (if _returnvalue_3
            (for _array_element_2 (`self.ManagedActors`) :!label _label
              (`/Engine/EditorBlueprintResources/StandardMacros.IsValid` _array_element_2
                (:`Is Valid`
                  (message `InteractInterface.OnInteract` _array_element_2 self))))
            (return true)
            (else
              (for _array_element_3 (`self.ManagedActors`)
                (`/Engine/EditorBlueprintResources/StandardMacros.IsValid` _array_element_3
                  (:`Is Valid`
                    (message `InteractInterface.ChainInteraction` _array_element_3 self))
                  (:`Is Not Valid`
                    (return false))))
              (return true)))))
      (else
        (`KismetSystemLibrary.PrintString` "This actor not in chain" false true (struct :`R` 1.0 :`G` 0.101327 :`A` 1.0))))
    (else
      (goto _label))))

(fn `SameColorCheck`
  (locals (bAnotherCheck :type Boolean))
  (bind _keys (`BlueprintMapLibrary.Map_Keys` (`self.InteractionChain`)))
  (for _array_element _keys :!label _label
    (if (`KismetSystemLibrary.IsValid` _array_element)
      (if (!= _array_element self)
        (if (`|EnumEquality` (`self.ColorEnumValue`) (`InteractActor.ColorEnumValue` _array_element))
          (set `self.ColorEnumValue` (cast `EObjectColor` (`KismetMathLibrary.Conv_IntToByte` (`KismetMathLibrary.RandomIntegerInRange` (`self.MinRandomIndex`) (`self.MaxRandomIndex`)))))
          (set `local.bAnotherCheck` true)
          (break)
          (else
            (set `local.bAnotherCheck` false)))
        (else
          (break)))))
  (if (`local.bAnotherCheck`)
    (goto _label)
    (else
      (return))))

(fn `UserConstructionScript`)