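; BP_Button is an interactable button that the player presses to get a success or error result.
; Interaction plays a player montage whose notify starts a timeline press and evaluates ResultInteraction, or forces failure when random success is enabled but not chosen.
; The result sets sound and message text, with failure also calling the game mode's ChangePlayerHealth.
; When another BP_BaseInteractActor is the caller, the button unhides itself instead.
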(event `InteractInterface.OnInteract`
  (params (Caller :type "Actor Object Reference"))
  (bind _asbp_player_character (cast `/Game/Blueprints/BP_PlayerCharacter` Caller)
    (:`then`
      (`|PlayMontage` (`Character.Mesh` _asbp_player_character) (`self.InteractionMontage`)
        (:`OnNotifyBegin`
          (`|ExecutionSequence`
            (:`then_0`
              (bind (_direction _pressalpha) (`Timeline|PushButton`)
                (:`Update`
                  (`SceneComponent.K2_SetRelativeLocation` (`self.Mesh`) (`KismetMathLibrary.VLerp` (0.0 0.0 0.0) (0.0 -15.0 0.0) _pressalpha) false false))))
            (:`then_1`
              (if (`self.isSuccessRandomly`)
                (if (`self.isRandomChoosen`)
                  (bind _result (`self.ResultInteraction` :!label _label))
                  (`self.CheckSuccess` _result)
                  (else
                    (`self.CheckSuccess` false)))
                (else
                  (goto _label))))))))
    (:`CastFailed`
      (cast `/Game/Blueprints/InteractActors/BP_BaseInteractActor` Caller
        (:`then`
          (`self.SetActorHiddenInGame` false))
        (:`CastFailed`
          (`KismetSystemLibrary.PrintString` "all cast failed" false true (struct :`R` 1.0 :`B` 0.045985 :`A` 1.0)))))))

(event `self.ReceiveBeginPlay`
  (`parent.ReceiveBeginPlay`))

(event `InteractInterface.ChainInteraction`
  (params (Caller :type "Actor Object Reference"))
  (`parent.ChainInteraction` Caller))

(event `CheckSuccess`
  (params (Condition :type Boolean))
  (`GameplayStatics.PlaySound2D` (select `bool` Condition :`false` "/Engine/EditorSounds/Notifications/CompileFailed_Cue.CompileFailed_Cue" :`true` "/Engine/VREditor/Sounds/UI/Click_on_Button_Cue.Click_on_Button_Cue" :!type "SoundBase Object Reference") 1.0 1.0 0.0 null null)
  (if Condition
    (`TextRenderComponent.K2_SetText` (`self.MessageText`) (`|FormatText` "Success"))
    (else
      (`SeverstalTestGameMode.ChangePlayerHealth` (`/Game/Blueprints/BP_MyFunctionLib.GetGameModeBP`) 1)
      (`TextRenderComponent.K2_SetText` (`self.MessageText`) (`|FormatText` "Error")))))

(fn `UserConstructionScript`
  (`parent.UserConstructionScript`))