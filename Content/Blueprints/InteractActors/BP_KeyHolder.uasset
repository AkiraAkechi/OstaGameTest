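; Interactable key holder that accepts a colored key from the player's inventory, colored at start along with its linked key actor.
; On interact, it takes the first inventory item and animates the key mesh into a socket.
; A color match shows the shield and, after chain checks pass, notifies managed actors.
; A mismatch changes player health, respawns the key as a pickup and resets the DoOnce for another attempt.
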(event `self.ReceiveBeginPlay`
  (bind _colorenumvalue (`self.ColorEnumValue`))
  (`parent.ReceiveBeginPlay`)
  (`KismetSystemLibrary.Delay` 0.2)
  (bind _keyactor (`self.KeyActor`)
    (:`then`
      (`/Game/Blueprints/InteractActors/BP_KeyPickUp.ChangeColor` _keyactor _colorenumvalue)
      (`PrimitiveComponent.SetMaterial` (`self.Mesh`) 0 (`BlueprintMapLibrary.Map_Find` (`self.MaterialMap`) _colorenumvalue)))
    (:`else`)))

(event `InteractInterface.OnInteract`
  (params (Caller :type "Actor Object Reference"))
  (bind _keymesh (`self.KeyMesh`))
  (bind _keymesh_2 (`self.KeyMesh`))
  (bind _keymesh_3 (`self.KeyMesh`))
  (bind (_returnvalue_location _returnvalue_rotation) (`KismetMathLibrary.BreakTransform` (`SceneComponent.GetSocketTransform` (`self.Mesh`) "KeySocket" "RTS_Actor")))
  (bind _returnvalue (`|EnumEquality` (`self.ColorEnumValue`) (`self.Key`)))
  (bind _asbp_player_character (cast `/Game/Blueprints/BP_PlayerCharacter` Caller))
  (if (`/Game/Blueprints/BP_PlayerCharacter.bGrabItem` _asbp_player_character)
    (`/Engine/EditorBlueprintResources/StandardMacros.DoOnce` false :!label _label
      (:`Completed`
        (bind _output_get (set `self.Key` (`|GetArrayItem` (`/Game/Blueprints/BP_PlayerCharacter.InventoryItems` _asbp_player_character))))
        (`/Game/Blueprints/BP_PlayerCharacter.DropItem` _asbp_player_character _output_get)
        (`PrimitiveComponent.SetMaterial` (`self.KeyMesh`) 0 (`BlueprintMapLibrary.Map_Find` (`self.MaterialMap`) (`self.Key`)))
        (`SceneComponent.SetHiddenInGame` _keymesh_2 false false)
        (`KismetSystemLibrary.MoveComponentTo` _keymesh_2 _returnvalue_location _returnvalue_rotation true true 1.0)
        (`GameplayStatics.PlaySound2D` (select `bool` _returnvalue :`false` "/Engine/EditorSounds/Notifications/CompileFailed_Cue.CompileFailed_Cue" :`true` "/Engine/VREditor/Sounds/UI/Click_on_Button_Cue.Click_on_Button_Cue" :!type "SoundBase Object Reference") 1.0 1.0 0.0 null null)
        (if _returnvalue
          (`SceneComponent.SetHiddenInGame` (`self.SphereShield`) false false)
          (bind _result (`self.ResultInteraction`))
          (if _result
            (bind _returnvalue_2 (`self.CompliteChainCheck`))
            (if _returnvalue_2
              (for _array_element (`self.ManagedActors`)
                (message `InteractInterface.ChainInteraction` _array_element self))))
          (else
            (`SeverstalTestGameMode.ChangePlayerHealth` (`/Game/Blueprints/BP_MyFunctionLib.GetGameModeBP`) 1)
            (bind _returnvalue_3 (`|SpawnActorFromClass` "/Game/Blueprints/InteractActors/BP_KeyPickUp.BP_KeyPickUp_C" (`KismetMathLibrary.MakeTransform` (`SceneComponent.K2_GetComponentLocation` _keymesh) (`SceneComponent.K2_GetComponentRotation` _keymesh)) "AdjustIfPossibleButAlwaysSpawn" "OverrideRootScale" null null))
            (`/Game/Blueprints/InteractActors/BP_KeyPickUp.ChangeColor` _returnvalue_3 (`self.Key`))
            (`SceneComponent.SetHiddenInGame` _keymesh_3 true false)
            (`SceneComponent.K2_SetRelativeLocation` _keymesh_3 (0.0 0.0 85.0) false false)
            (goto _label :!via `Reset`)))))
    (else
      (`/Game/Blueprints/BP_MyFunctionLib.Print Screen Message` "Need to put something here" 5.0))))

(fn `UserConstructionScript`
  (`parent.UserConstructionScript`))