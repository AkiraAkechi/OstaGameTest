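; BP_KeyPickUp is a color-coded key pickup whose mesh material comes from a color-to-material map.
; When the player interacts, it stops its interp movement and plays an interaction montage, whose notify adds the color via PickUpItem and destroys the key.
; If GrabItem is set, a six-slot inventory limit and DoOnce gate the pickup.
; Interaction from another BP_BaseInteractActor unhides the key instead.
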(event `ChangeColor`
  (params (Color :type "EObjectColor Enum (by ref)"))
  (set `self.ColorEnumValue` Color)
  (`PrimitiveComponent.SetMaterial` (`self.Mesh`) 0 (`BlueprintMapLibrary.Map_Find` (`self.MaterialMap`) Color)))

(event `InteractInterface.OnInteract`
  (params (Caller :type "Actor Object Reference"))
  (bind _asbp_player_character (cast `/Game/Blueprints/BP_PlayerCharacter` Caller)
    (:`then`
      (if (`/Game/Blueprints/BP_PlayerCharacter.bGrabItem` _asbp_player_character)
        (if (< (`KismetArrayLibrary.Array_Length` (`/Game/Blueprints/BP_PlayerCharacter.InventoryItems` _asbp_player_character)) 6)
          (`/Engine/EditorBlueprintResources/StandardMacros.DoOnce` false
            (:`Completed`
              (`MovementComponent.StopMovementImmediately` (`self.InterpToMovement`) :!label _label)
              (`|PlayMontage` (`Character.Mesh` _asbp_player_character) (`self.InteractionMontage`)
                (:`OnNotifyBegin`
                  (`PrimitiveComponent.SetCollisionEnabled` (`self.Mesh`) "NoCollision")
                  (`/Game/Blueprints/BP_PlayerCharacter.PickUpItem` _asbp_player_character (`self.ColorEnumValue`))
                  (`self.K2_DestroyActor`)))))
          (else
            (`/Game/Blueprints/BP_MyFunctionLib.Print Screen Message` "Cant Pick up \nAll item slots is full" 5.0)))
        (else
          (goto _label))))
    (:`CastFailed`
      (cast `/Game/Blueprints/InteractActors/BP_BaseInteractActor` Caller)
      (`self.SetActorHiddenInGame` false))))

(fn `UserConstructionScript`
  (`parent.UserConstructionScript`))